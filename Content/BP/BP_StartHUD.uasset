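; BP_StartHUD sets up the game's start screen when play begins.
; BeginPlay creates the BP_StartScreen widget, adds it to the viewport, and switches the first player controller to UI-only input with a visible mouse cursor.
; It then fills the widget's latest score and record texts once from the stats subsystem's LatestScore and BestScore.
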(event `self.ReceiveBeginPlay`
  (bind _returnvalue (`GameplayStatics.GetPlayerController` 0))
  (bind _returnvalue_2 (subsystem `StatsSubsystem`))
  (bind _startwidget (`self.StartWidget`))
  (bind _returnvalue_3 (`|CreateWidget` "/Game/BP/BP_StartScreen.BP_StartScreen_C"))
  (bind _output_get (set `self.StartWidget` _returnvalue_3))
  (`UserWidget.AddToViewport` _output_get 0)
  (`WidgetBlueprintLibrary.SetInputMode_UIOnlyEx` _returnvalue null)
  (set `PlayerController.bShowMouseCursor` true _returnvalue)
  (set `EditableTextBox.Text` (`KismetTextLibrary.Conv_IntToText` (`StatsSubsystem.LatestScore` _returnvalue_2)) (`/Game/BP/BP_StartScreen.LatestScoreValue` _startwidget))
  (set `EditableTextBox.Text` (`KismetTextLibrary.Conv_IntToText` (`StatsSubsystem.BestScore` _returnvalue_2)) (`/Game/BP/BP_StartScreen.RecordValue` _startwidget)))

(fn `UserConstructionScript`)