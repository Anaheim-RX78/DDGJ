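; Damageable prop that can explode when it dies, hurting everything around it.
; On death, an explosive prop runs a multi-sphere Visibility trace at its location and sends very high explosive damage to hit actors implementing DamageInterface.
; It clears its Explosive flag before tracing, so it detonates only once even if blasts chain back to it.
; The trace still draws timed debug shapes.
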(event `self.OnDeath`
  (bind _returnvalue (`self.K2_GetActorLocation`))
  (if (`self.Explosive`)
    (set `self.Explosive` false)
    (bind (_outhits _returnvalue_2) (`KismetSystemLibrary.SphereTraceMulti` :`Start` _returnvalue :`End` _returnvalue :`Radius` (`self.ExplodeRadius`) :`TraceChannel` "TraceTypeQuery1" :`DrawDebugType` "ForDuration"))
    (if _returnvalue_2
      (for _array_element _outhits
        (bind (_bblockinghit _binitialoverlap _time _distance _location _impactpoint _normal _impactnormal _physmat _hitactor) (`GameplayStatics.BreakHitResult` _array_element))
        (if (`KismetSystemLibrary.DoesImplementInterface` _hitactor "/Script/DDGJ.DamageInterface")
          (message `DamageInterface.DoDamage` _hitactor 10000.0 true))))))

(fn `UserConstructionScript`)